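; BP_Parallax is a scrolling background plane that follows BP_MainCharacter to fake parallax as the character moves along X.
; On BeginPlay it attaches itself to the character, keeping world rotation and scale, and creates a dynamic material for its Plane.
; Each tick it accumulates an offset at ParallaxSpeed, using only the direction of X velocity, and feeds the material's Offset parameter.
; The offset wraps only when it exceeds 1.
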(event `self.ReceiveBeginPlay`
  (bind _plane (`self.Plane`))
  (bind _returnvalue (`GameplayStatics.GetActorOfClass` "/Game/Blueprints/Player/Game/General/BP_MainCharacter.BP_MainCharacter_C"))
  (bind _output_get (set `self.MainCharacter` _returnvalue))
  (`self.K2_AttachToActor` _output_get "None" "KeepRelative" "KeepWorld" "KeepWorld")
  (bind _returnvalue_2 (`PrimitiveComponent.CreateDynamicMaterialInstance` _plane 0 (`PrimitiveComponent.GetMaterial` _plane 0) "None"))
  (set `self.DynamicMaterial` _returnvalue_2))

(event `self.ReceiveTick`
  (params (DeltaSeconds :type "Float (single-precision)"))
  (bind _returnvalue_x (`KismetMathLibrary.BreakVector` (`self.GetVelocity` (`self.MainCharacter`))))
  (bind _returnvalue_x_2 (`KismetMathLibrary.BreakVector` (`self.GetVelocity` (`self.MainCharacter`))))
  (`/Engine/EditorBlueprintResources/StandardMacros.IsValid` (`self.MainCharacter`)
    (:`Is Valid`
      (set `self.Delta` (* DeltaSeconds (`KismetMathLibrary.VSize` (* (`KismetMathLibrary.Vector_Normal2D` (`KismetMathLibrary.MakeVector` _returnvalue_x)) (`self.ParallaxSpeed`)))))
      (if (not (> _returnvalue_x_2 0.0))
        (`/Engine/EditorBlueprintResources/StandardMacros.NegateFloat` (`self.Delta`)
          (:`  `
            _)))
      (bind _output_get (set `self.CurrentOffset` (+ (`self.CurrentOffset`) (`self.Delta`))))
      (if (> _output_get 1.0)
        (set `self.CurrentOffset` (`KismetMathLibrary.FMod` (`self.CurrentOffset`) 1.0)))
      (`MaterialInstanceDynamic.SetScalarParameterValue` (`self.DynamicMaterial`) "Offset" (`self.CurrentOffset`)))))

(fn `UserConstructionScript`)