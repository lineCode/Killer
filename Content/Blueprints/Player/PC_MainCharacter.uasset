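; Player controller for the main character that handles pausing and shoot input.
; On begin play it sets game-only input and hides the cursor.
; The Pause action toggles the paused state, creating a new pause menu widget with game-and-UI input and a visible cursor, or removing it and restoring game-only input.
; The Shoot action calls the OnShoot event dispatcher.
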(event `self.ReceiveBeginPlay`
  ;[1 1 1] Begin Play
  (`WidgetBlueprintLibrary.SetInputMode_GameOnly` self)
  (set `self.bShowMouseCursor` false))

(event `InputAction|Pause` :paused true
  (params (Key :type "Key Structure"))
  (bind _pausemenuwidget (`self.PauseMenuWidget`))
  (:`Pressed`
    (if (`GameplayStatics.IsGamePaused`)
      ;[1 1 1] Unpause Game
      (`GameplayStatics.SetGamePaused` false)
      (`/Engine/EditorBlueprintResources/StandardMacros.IsValid` _pausemenuwidget
        (:`Is Valid`
          (`Widget.RemoveFromParent` _pausemenuwidget)
          (`WidgetBlueprintLibrary.SetInputMode_GameOnly` self)
          (set `self.bShowMouseCursor` false)))
      (else
        ;[1 1 1] Pause Game
        (`GameplayStatics.SetGamePaused` true)
        (bind _returnvalue (`|CreateWidget` "/Game/Blueprints/Widgets/Menu/WBP_PauseMenu.WBP_PauseMenu_C" self))
        (bind _output_get (set `self.PauseMenuWidget` _returnvalue))
        (`UserWidget.AddToViewport` _output_get 0)
        (`WidgetBlueprintLibrary.SetInputMode_GameAndUIEx` self null "DoNotLock" false)
        (set `self.bShowMouseCursor` true)))))

(event `InputAction|Shoot` :consume false :overrideparent false
  (params (Key :type "Key Structure"))
  (:`Pressed`
    (`self.OnShoot`)))

(fn `UserConstructionScript`)