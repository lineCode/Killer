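; Player character for a 2D side-scroller, with flipbook animation, music playback and camera effects.
; Tick picks idle, run or jump flipbooks, flips the sprite, pins the actor to the XZ plane and drives walk particles with Delay-throttled footsteps.
; Music envelope pulses the orthographic camera width, scaled by saved shake and inversely by volume.
; It also handles hard-landing feedback, HUD death notification and timeline-driven camera moves.
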(event `self.ReceiveBeginPlay`
  ;[1 1 1] Begin Play
  (`PlayerCameraManager.StartCameraShake` :`self` (`GameplayStatics.GetPlayerCameraManager` 0) :`ShakeClass` "/Game/Blueprints/CameraShakes/CS_Rotate.CS_Rotate_C")
  (`self.PlayMusic`)
  (bind _returnvalue (`NiagaraFunctionLibrary.SpawnSystemAttached` "/Game/Graphics/Particles/NS_Walk.NS_Walk" (`self.CapsuleComponent`) "None" (0.0 0.0 -70.0) (struct) "KeepRelativeOffset" false false))
  (set `self.WalkNiagaraSystem` _returnvalue)
  (set `self.StartFOV` (`CameraComponent.OrthoWidth` (`self.Camera`)))
  (bind _save (`/Game/Blueprints/Settings/FL_General.GetSave`))
  (`/Engine/EditorBlueprintResources/StandardMacros.IsValid` _save
    (:`Is Valid`
      (`self.OnAudioSettingsChanged` (`Save.FOVShake` _save) (`Save.MusicVolume` _save)))
    (:`Is Not Valid`
      _))
  (`/Game/Blueprints/Settings/FL_General.ApplySoundSettings`))

(event `self.ReceiveTick`
  (params (DeltaSeconds :type "Float (single-precision)"))
  (bind (_returnvalue_x _returnvalue_y _returnvalue_z) (`KismetMathLibrary.BreakVector` (`self.K2_GetActorLocation`)))
  ;[1 1 1] Tick
  (`self.UpdateAnimation`)
  (`self.RotateCharacter`)
  (`self.K2_SetActorLocation` (`KismetMathLibrary.MakeVector` _returnvalue_x 0.0 _returnvalue_z))
  (`self.SpawnWalkParticlesAndPlaySound`))

(event `self._OnKilled`
  (params (InstigatedBy :type "Controller Object Reference") (DamageCauser :type "Actor Object Reference"))
  ;[1 1 1] On Killed
  (bind _asplayer_controller (cast `PlayerController` (`self.GetController`)))
  (bind _ashud_player (cast `/Game/Blueprints/Player/HUD_Player` (`PlayerController.GetHUD` _asplayer_controller)))
  (`/Game/Blueprints/Widgets/HUD/WBP_PlayerHUD.OnPlayerKilled` (`/Game/Blueprints/Player/HUD_Player.PlayerHUDWidget` _ashud_player)))

(event `self.OnLanded`
  (params (Hit :type "HitResult Structure (by ref)"))
  (bind (_returnvalue_x _returnvalue_y _returnvalue_z) (`KismetMathLibrary.BreakVector` (`self.GetVelocity`)))
  ;[1 1 1] On Landed
  (if (>= (`KismetMathLibrary.Abs` _returnvalue_z) (`self.OnLandedImpactSpeed`))
    (`GameplayStatics.PlaySoundAtLocation` "/Game/Sounds/Effects/Game/Bone_Crack.Bone_Crack" (`self.K2_GetActorLocation`) (struct) 1.0 (`KismetMathLibrary.RandomFloatInRange` 0.9 1.1) 0.0 null null null null)
    (`NiagaraFunctionLibrary.SpawnSystemAtLocation` "/Game/Graphics/Particles/NS_OnLanded.NS_OnLanded" (`self.K2_GetActorLocation`))
    (`PlayerCameraManager.StartCameraShake` :`self` (`GameplayStatics.GetPlayerCameraManager` 0) :`ShakeClass` "/Game/Blueprints/CameraShakes/CS_OnLanded.CS_OnLanded_C")))

(event `PlayFootstepSound`
  ;[1 1 1] Footstep Sound
  (`KismetSystemLibrary.Delay` 0.2)
  (if (not (`NavMovementComponent.IsFalling` (`self.CharacterMovement`)))
    (`GameplayStatics.PlaySoundAtLocation` "/Game/Sounds/Effects/Game/Footstep_Cue.Footstep_Cue" (`self.K2_GetActorLocation`) (struct) 1.0 1.0 0.0 null null null null)))

(event `self.AudioComp.OnAudioSingleEnvelopeValue`
  (params (PlayingSoundWave :type "SoundWave Object Reference") (EnvelopeValue :type "Float (single-precision)"))
  (`self.ChangeFOVOnMusicEnvelope` EnvelopeValue))

(event `MoveCameraToNewLocation`
  (params (Position :type "Vector Structure"))
  (bind (_returnvalue_x _returnvalue_y _returnvalue_z) (`KismetMathLibrary.BreakVector` (`SceneComponent.K2_GetComponentLocation` (`self.Camera`))))
  (bind (_direction _deltatime) (`Timeline|CameraMove` :!via `PlayFromStart`)
    (:`Update`
      (`SceneComponent.K2_SetWorldLocation` (`self.Camera`) (`KismetMathLibrary.VInterpTo` (`KismetMathLibrary.MakeVector` _returnvalue_x _returnvalue_y _returnvalue_z) (`KismetMathLibrary.MakeVector` Position_X _returnvalue_y Position_Z) _deltatime 0.1) false false))))

(fn `ChangeFOVOnMusicEnvelope`
  (params (EnvelopeValue :type "Float (double-precision)"))
  (set `CameraComponent.OrthoWidth` (`KismetMathLibrary.FInterpTo` (`CameraComponent.OrthoWidth` (`self.Camera`)) (- (`self.StartFOV`) (* EnvelopeValue (`self.OnAudioEnvelopeMultiplier`))) (`GameplayStatics.GetWorldDeltaSeconds`) 10.0) (`self.Camera`)))

(fn `OnAudioSettingsChanged`
  (params (FOVShake :type "Float (double-precision)") (MusicVolume :type "Float (double-precision)"))
  (if (`KismetMathLibrary.NearlyEqual_FloatFloat` MusicVolume 0.0 0.01)
    (set `self.OnAudioEnvelopeMultiplier` 0.0)
    (else
      (set `self.OnAudioEnvelopeMultiplier` (* (* FOVShake 50000.0) (/ 1.0 (`KismetMathLibrary.FClamp` MusicVolume 0.001)))))))

(fn `PlayMusic`
  (bind _audiocomp (`self.AudioComp`))
  (bind _musictoplay (`self.MusicToPlay`))
  (`/Engine/EditorBlueprintResources/StandardMacros.IsValid` _musictoplay
    (:`Is Valid`
      (`AudioComponent.SetSound` _audiocomp _musictoplay)
      (`AudioComponent.Play` _audiocomp 0.0))))

(fn `ReturnCameraToDefaultLocation`
  (`self.MoveCameraToNewLocation` (`SceneComponent.K2_GetComponentLocation` (`self.SpringArm`))))

(fn `RotateCharacter`
  (bind _velocity_x (`KismetMathLibrary.BreakVector` (`MovementComponent.Velocity` (`self.CharacterMovement`))))
  (`/Engine/EditorBlueprintResources/StandardMacros.CompareFloat` _velocity_x
    (:`>`
      (`SceneComponent.K2_SetWorldRotation` :`self` (`self.Sprite`)))
    (:`<`
      (`SceneComponent.K2_SetWorldRotation` (`self.Sprite`) (struct :`Yaw` 180.0) false false))))

(fn `SpawnWalkParticlesAndPlaySound`
  (bind _returnvalue_x (`KismetMathLibrary.BreakVector` (`self.GetVelocity`)))
  (bind _walkniagarasystem (`self.WalkNiagaraSystem`))
  (if (and (`CharacterMovementComponent.IsWalking` (`self.CharacterMovement`)) (>= (`KismetMathLibrary.Abs` _returnvalue_x) (`self.SpeedForWalkParticles`)))
    (`/Engine/EditorBlueprintResources/StandardMacros.IsValid` _walkniagarasystem
      (:`Is Valid`
        (`ActorComponent.Activate` _walkniagarasystem false)
        (`self.PlayFootstepSound`)))
    (else
      (`/Engine/EditorBlueprintResources/StandardMacros.IsValid` (`self.WalkNiagaraSystem`)
        (:`Is Valid`
          (`ActorComponent.Deactivate` _walkniagarasystem))))))

(fn `UpdateAnimation`
  (`PaperFlipbookComponent.SetFlipbook` (`self.Sprite`) (select `bool` (`NavMovementComponent.IsFalling` (`self.CharacterMovement`)) :`false` (select `bool` (> (`KismetMathLibrary.VSize` (`MovementComponent.Velocity` (`self.CharacterMovement`))) 0.0) :`false` "/Game/Graphics/Animations/Player/Idle/FB_Killer_Idle.FB_Killer_Idle" :`true` "/Game/Graphics/Animations/Player/Run/FB_Killer_Run.FB_Killer_Run" :!type "PaperFlipbook Object Reference") :`true` "/Game/Graphics/Animations/Player/Jump/FB_Killer_Jump.FB_Killer_Jump")))

(fn `UserConstructionScript`)