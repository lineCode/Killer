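; Player controller for the main menu that shows the mouse cursor and accepts both game and UI input from BeginPlay.
; Pressing Escape gathers all WBP_Menu widgets, including nested ones, and walks the list in reverse.
; It calls Return on the first one found in the viewport, using a HasReturned flag so only one menu responds per press.
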(event `self.ReceiveBeginPlay`
  (`WidgetBlueprintLibrary.SetInputMode_GameAndUIEx` self null)
  (set `self.bShowMouseCursor` true))

(event `Key|Escape`
  (params (Key :type "Key Structure"))
  (:`Pressed`
    (set `self.HasReturned` false)
    (bind _foundwidgets (`WidgetBlueprintLibrary.GetAllWidgetsOfClass` "/Game/Blueprints/Widgets/Menu/General/WBP_Menu.WBP_Menu_C" false))
    (bind (_arrayindex _arrayelement) (`/Engine/EditorBlueprintResources/StandardMacros.ReverseForEachLoop` _foundwidgets)
      (:`LoopBody`
        (if (`self.HasReturned`)
          _
          (elif (`Widget.IsInViewport` _arrayelement)
            (`/Game/Blueprints/Widgets/Menu/General/WBP_Menu.Return` _arrayelement)
            (set `self.HasReturned` true)))))))

(fn `UserConstructionScript`)