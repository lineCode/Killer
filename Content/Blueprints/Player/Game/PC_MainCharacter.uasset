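; PC_MainCharacter is the player controller that handles the pause menu and shoot input for the main character.
; The Pause action toggles game pause, creating or removing WBP_PauseMenu while switching the input mode and mouse cursor.
; A positive Shoot axis value calls OnShoot, likely an event dispatcher, on every frame the input is held.
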(event `InputAction|Pause` :paused true
  (params (Key :type "Key Structure"))
  (bind _pausemenuwidget (`self.PauseMenuWidget`))
  ;[1 1 1] Pause Menu
  (:`Pressed`
    (if (`GameplayStatics.IsGamePaused`)
      ;;[1 1 1] Unpause Game
      (`GameplayStatics.SetGamePaused` false)
      (`/Engine/EditorBlueprintResources/StandardMacros.IsValid` _pausemenuwidget
        (:`Is Valid`
          (`Widget.RemoveFromParent` _pausemenuwidget)
          (`WidgetBlueprintLibrary.SetInputMode_GameOnly` self)
          (set `self.bShowMouseCursor` false)))
      (else
        ;;[1 1 1] Pause Game
        (`GameplayStatics.SetGamePaused` true)
        (bind _returnvalue (`|CreateWidget` "/Game/Blueprints/Widgets/Menu/Pause/WBP_PauseMenu.WBP_PauseMenu_C" self))
        (bind _output_get (set `self.PauseMenuWidget` _returnvalue))
        (`UserWidget.AddToViewport` _output_get 0)
        (`WidgetBlueprintLibrary.SetInputMode_GameAndUIEx` self null "DoNotLock" false)
        (set `self.bShowMouseCursor` true)))))

(event `InputAxis|Shoot`
  (params (AxisValue :type "Float (single-precision)"))
  ;[1 1 1] Shoot Event
  (if (> AxisValue 0.0)
    (`self.OnShoot`)))

(fn `UserConstructionScript`)