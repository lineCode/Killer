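; BP_MainCharacter is the player character that owns the orthographic camera and music playback, starting a rotating camera shake and music on BeginPlay.
; The music's envelope drives a smoothed OrthoWidth pulse, scaled by the saved FOV shake setting and inversely by music volume, and disabled near zero volume.
; A timeline eases the camera along X and Z to a requested position or back to the spring arm.
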(event `self.ReceiveBeginPlay`
  (bind _returnvalue (`Save.GetSave`))
  ;[1 1 1] Camera Shake
  (bind _asplayer_controller (cast `PlayerController` (`self.GetController`))
    (:`then`
      (`PlayerCameraManager.StartCameraShake` :`self` (`PlayerController.PlayerCameraManager` _asplayer_controller) :`ShakeClass` "/Game/Blueprints/Effects/CameraShakes/CS_Rotate.CS_Rotate_C"))
    (:`CastFailed`
      _))
  ;[1 1 1] Start Music
  (`self.PlayMusic`)
  ;[1 1 1] Audio
  (set `self.StartFOV` (`CameraComponent.OrthoWidth` (`self.CameraComponent`)))
  (`self.OnAudioSettingsChanged` (`Save.FOVShake` _returnvalue) (`Save.MusicVolume` _returnvalue))
  (`/Game/Blueprints/General/FunctionLibraries/FL_General.ApplySoundSettings`))

(event `self.AudioComponent.OnAudioSingleEnvelopeValue`
  (params (PlayingSoundWave :type "SoundWave Object Reference") (EnvelopeValue :type "Float (single-precision)"))
  ;[1 1 1] Music Camera FOV
  (`self.Change FOV on Music Envelope` EnvelopeValue))

(event `MoveCameraToNewLocation`
  (params (Position :type "Vector Structure"))
  (bind _returnvalue (`SceneComponent.K2_GetComponentLocation` (`self.CameraComponent`)))
  (bind (_direction _deltatime) (`Timeline|DeltaTimeTimeline` :!via `PlayFromStart`)
    (:`Update`
      (`SceneComponent.K2_SetWorldLocation` (`self.CameraComponent`) (`KismetMathLibrary.VInterpTo` _returnvalue (`KismetMathLibrary.MakeVector` (.x Position) (`.Y` (`KismetMathLibrary.BreakVector3f` _returnvalue)) (.z Position)) _deltatime 0.1) false false))))

(fn `Change FOV on Music Envelope`
  (params (EnvelopeValue :type "Float (double-precision)"))
  (set `CameraComponent.OrthoWidth` (`KismetMathLibrary.FInterpTo` (`CameraComponent.OrthoWidth` (`self.CameraComponent`)) (- (`self.StartFOV`) (* EnvelopeValue (`self.AudioEnvelopeMultiplier`))) (`GameplayStatics.GetWorldDeltaSeconds`) 10.0) (`self.CameraComponent`)))

(fn `OnAudioSettingsChanged`
  (params (FOVShake :type "Float (double-precision)") (MusicVolume :type "Float (double-precision)"))
  (if (`KismetMathLibrary.NearlyEqual_FloatFloat` MusicVolume 0.0 0.01)
    (set `self.AudioEnvelopeMultiplier` 0.0)
    (else
      (set `self.AudioEnvelopeMultiplier` (* (* FOVShake 50000.0) (/ 1.0 (`KismetMathLibrary.FClamp` MusicVolume 0.001)))))))

(fn `PlayMusic`
  (bind _audiocomponent (`self.AudioComponent`))
  (bind _musictoplay (`self.MusicToPlay`))
  (`/Engine/EditorBlueprintResources/StandardMacros.IsValid` _musictoplay
    (:`Is Valid`
      (`AudioComponent.SetSound` _audiocomponent _musictoplay)
      (`AudioComponent.Play` _audiocomponent 0.0))))

(fn `ReturnCameraToDefaultLocation`
  (`self.MoveCameraToNewLocation` (`SceneComponent.K2_GetComponentLocation` (`self.SpringArmComponent`))))

(fn `UserConstructionScript`)