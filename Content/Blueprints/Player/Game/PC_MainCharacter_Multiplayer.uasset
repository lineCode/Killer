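; PC_MainCharacter_Multiplayer is a player controller for the multiplayer main character that handles the pause menu.
; The Pause input toggles an IsPaused flag, creating and showing a WBP_PauseMenu widget or removing it.
; Each toggle also switches between game-and-UI and game-only input modes and shows or hides the cursor, without pausing the game simulation itself.
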(event `InputAction|Pause` :paused true
  (params (Key :type "Key Structure"))
  (bind _pausemenuwidget (`self.PauseMenuWidget`))
  ;[1 1 1] Pause Menu
  (:`Pressed`
    (if (`self.IsPaused`)
      ;;[1 1 1] Unpause Game
      (`/Engine/EditorBlueprintResources/StandardMacros.IsValid` _pausemenuwidget
        (:`Is Valid`
          (`Widget.RemoveFromParent` _pausemenuwidget)
          (`WidgetBlueprintLibrary.SetInputMode_GameOnly` self)
          (set `self.bShowMouseCursor` false)
          (set `self.IsPaused` false)))
      (else
        ;;[1 1 1] Pause Game
        (bind _returnvalue (`|CreateWidget` "/Game/Blueprints/Widgets/Menu/Pause/WBP_PauseMenu.WBP_PauseMenu_C" self))
        (bind _output_get (set `self.PauseMenuWidget` _returnvalue))
        (`UserWidget.AddToViewport` _output_get 0)
        (`WidgetBlueprintLibrary.SetInputMode_GameAndUIEx` self null "DoNotLock" false)
        (set `self.bShowMouseCursor` true)
        (set `self.IsPaused` true)))))

(fn `UserConstructionScript`)