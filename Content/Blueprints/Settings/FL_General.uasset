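; General function library whose GetSave function returns the game's BP_Save save object.
; It creates a fresh BP_Save to read the slot name, writes it to that slot if no save exists, then loads and casts the slot.
; If loading or casting fails, it overwrites the slot with the fresh object and returns that instead.
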(fn `GetSave`
  (returns (Save :type "/Game/Blueprints/Settings/BP_Save Object Reference"))
  (bind _returnvalue (`GameplayStatics.CreateSaveGameObject` "/Game/Blueprints/Settings/BP_Save.BP_Save_C"))
  (`/Engine/EditorBlueprintResources/StandardMacros.IsValid` _returnvalue
    (:`Is Valid`
      (bind _returnvalue_2 (`GameplayStatics.DoesSaveGameExist` (`Save.SlotName` _returnvalue)))
      (if (not _returnvalue_2)
        (`GameplayStatics.SaveGameToSlot` _returnvalue (`Save.SlotName` _returnvalue)))
      (bind _returnvalue_3 (`GameplayStatics.LoadGameFromSlot` (`Save.SlotName` _returnvalue)))
      (`/Engine/EditorBlueprintResources/StandardMacros.IsValid` _returnvalue_3
        (:`Is Valid`
          (bind _asbp_save (cast `/Game/Blueprints/Settings/BP_Save` _returnvalue_3)
            (:`then`
              (return _asbp_save))
            (:`CastFailed`
              _)))
        (:`Is Not Valid`
          _))
      (`GameplayStatics.SaveGameToSlot` _returnvalue (`Save.SlotName` _returnvalue))
      (return _returnvalue))))